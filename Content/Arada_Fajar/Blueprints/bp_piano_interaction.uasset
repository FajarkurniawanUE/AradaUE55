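; Piano interaction Blueprint that plays the next sound from an array, wrapping around, each time Interact is released.
; Tick checks whether the pc_arada controller's CurrentTracingActor is the piano mesh, enabling this actor's input while it is and disabling it otherwise.
; Paired DoOnce gates limit the custom-depth highlight and Umg_interior interact prompt updates to changes in trace state.
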(event `beingTrace`
  (`self.EnableInput` (`GameplayStatics.GetPlayerController` 0))
  (`|ExecutionSequence`
    (:`then_0`
      (`/Engine/EditorBlueprintResources/StandardMacros.DoOnce` false :!label _label
        (:`Completed`
          (bind _foundwidgets (`WidgetBlueprintLibrary.GetAllWidgetsOfClass` "/Game/Arada_Fajar/Blueprints/umg_interior.umg_interior_C" false))
          (bind _output (`|GetArrayItem` _foundwidgets))
          (`/Game/Arada_Fajar/Blueprints/umg_interior.show_interact` _output "SelfHitTestInvisible")
          (`PrimitiveComponent.SetRenderCustomDepth` (`StaticMeshActor.StaticMeshComponent` (`self.Piano SM`)) true)
          (set `/Game/Arada_Fajar/Blueprints/umg_interior.LookingAtDoor` false _output))))
    (:`then_1`
      (goto _label_2 :!via `Reset`))))

(event `notTrace`
  (`self.DisableInput` (`GameplayStatics.GetPlayerController` 0))
  (`|ExecutionSequence`
    (:`then_0`
      (goto _label :!via `Reset`))
    (:`then_1`
      (`/Engine/EditorBlueprintResources/StandardMacros.DoOnce` false :!label _label_2
        (:`Completed`
          (bind _foundwidgets (`WidgetBlueprintLibrary.GetAllWidgetsOfClass` "/Game/Arada_Fajar/Blueprints/umg_interior.umg_interior_C" false))
          (`/Game/Arada_Fajar/Blueprints/umg_interior.show_interact` (`|GetArrayItem` _foundwidgets) "Collapsed")
          (`PrimitiveComponent.SetRenderCustomDepth` (`StaticMeshActor.StaticMeshComponent` (`self.Piano SM`)) false))))))

(event `self.ReceiveTick`
  (params (DeltaSeconds :type "Float (single-precision)"))
  (bind _asstatic_mesh_actor (cast `StaticMeshActor` (`/Game/Arada_Fajar/Blueprints/pc_arada.CurrentTracingActor` (`self.As Pc Arada`)))
    (:`then`
      (if (== _asstatic_mesh_actor (`self.Piano SM`))
        (`self.beingTrace`)
        (else
          (`self.notTrace` :!label _label_3))))
    (:`CastFailed`
      (goto _label_3))))

(event `self.ReceiveBeginPlay`
  (`|ExecutionSequence`
    (:`then_0`
      (bind _foundwidgets (`WidgetBlueprintLibrary.GetAllWidgetsOfClass` "/Game/Arada_Fajar/Blueprints/umg_orbital.umg_orbital_C" false))
      (set `self.umg_orbital` (`|GetArrayItem` _foundwidgets)))
    (:`then_1`
      (bind _aschar_arada_interior (cast `/Game/Arada_Fajar/Blueprints/char_arada_interior` (`GameplayStatics.GetPlayerCharacter` 0)))
      (set `self.As Char Arada Interior` _aschar_arada_interior))
    (:`then_2`
      (bind _aspc_arada (cast `/Game/Arada_Fajar/Blueprints/pc_arada` (`GameplayStatics.GetPlayerController` 0)))
      (set `self.As Pc Arada` _aspc_arada))))

(event `InputAction|Interact`
  (params (Key :type "Key Structure"))
  (:`Released`
    (`self.playPiano`)))

(event `playPiano`
  (bind _audio (`self.Audio`))
  (`AudioComponent.SetSound` _audio (`|GetArrayItem` (`self.Sounds`) (`self.soundIndex`)))
  (`AudioComponent.Play` _audio 0.0)
  (if (>= (`self.soundIndex`) (`KismetArrayLibrary.Array_LastIndex` (`self.Sounds`)))
    (set `self.soundIndex` 0)
    (else
      (`/Engine/EditorBlueprintResources/StandardMacros.IncrementInt` (`self.soundIndex`)))))

(fn `UserConstructionScript`)