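; BP_carsRandomizer is a car actor that gives itself a random model and paint color.
; The construction script picks a random skeletal mesh from CarsArray and assigns it to the SkeletalMesh component.
; It then creates a dynamic material instance of slot 0 and sets its Color parameter from a random entry in Colors.
; All logic runs at construction, and the event graph is empty.
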(fn `UserConstructionScript`
  (bind _skeletalmesh (`self.SkeletalMesh`))
  (`SkeletalMeshComponent.SetSkeletalMeshAsset` (`self.SkeletalMesh`) (`KismetArrayLibrary.Array_Random` (`self.CarsArray`)))
  (bind _returnvalue (`PrimitiveComponent.CreateDynamicMaterialInstance` _skeletalmesh 0 (`PrimitiveComponent.GetMaterial` _skeletalmesh 0) "None"))
  (`MaterialInstanceDynamic.SetVectorParameterValue` _returnvalue "Color" (`KismetArrayLibrary.Array_Random` (`self.Colors`)))
  (`PrimitiveComponent.SetMaterial` (`self.SkeletalMesh`) 0 _returnvalue))