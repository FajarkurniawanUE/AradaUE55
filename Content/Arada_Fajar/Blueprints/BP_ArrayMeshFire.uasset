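; Spline-based actor that lays an array of meshes along a path in its construction script, apparently for fire, with random height at each segment end.
; With UniformLength on, it places random meshes from a list at fixed length intervals, clamping tangents to that length.
; Otherwise it spans each pair of spline points with one collidable mesh, using a dynamic sequence material with randomized Speed.
; The event graph is empty.
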(fn `UserConstructionScript`
  (bind _spline (`self.Spline`))
  (bind _spline_2 (`self.Spline`))
  (bind _spline_3 (`self.Spline`))
  (bind _meshes (`self.Meshes`))
  (bind _cablesize (`self.cableSize`))
  (bind _returnvalue (`KismetMathLibrary.MakeVector2D` (`self.Width`) (`KismetMathLibrary.RandomFloatInRange` (`self.Height min`) (`self.Height max`))))
  (bind _returnvalue_2 (`KismetMathLibrary.MakeVector2D` (`self.Width`) (`KismetMathLibrary.RandomFloatInRange` (`self.Height min`) (`self.Height max`))))
  (bind _returnvalue_3 (`KismetMathLibrary.FTrunc` (/ (`SplineComponent.GetSplineLength` (`self.Spline`)) (`self.MeshLength`))))
  (if (`self.Uniform Length`)
    (if (> _returnvalue_3 0)
      (for _index (range _returnvalue_3)
        (bind _returnvalue_4 (`AddComponent|NODE_AddSplineMeshComponent-2`))
        (`StaticMeshComponent.SetStaticMesh` _returnvalue_4 (`|GetArrayItem` _meshes (`KismetMathLibrary.RandomIntegerInRange` 0 (`KismetArrayLibrary.Array_LastIndex` _meshes))))
        (`SplineMeshComponent.SetStartScale` _returnvalue_4 _returnvalue true)
        (`SplineMeshComponent.SetEndScale` _returnvalue_4 _returnvalue true)
        (bind _returnvalue_5 (* _index (`self.MeshLength`)))
        (bind _returnvalue_6 (* (+ _index 1) (`self.MeshLength`)))
        (`SplineMeshComponent.SetStartAndEnd` _returnvalue_4 (`SplineComponent.GetLocationAtDistanceAlongSpline` _spline_3 _returnvalue_5 "Local") (`KismetMathLibrary.ClampVectorSize` (`SplineComponent.GetTangentAtDistanceAlongSpline` _spline_3 _returnvalue_5 "Local") 0.0 (`self.MeshLength`)) (`SplineComponent.GetLocationAtDistanceAlongSpline` _spline_2 _returnvalue_6 "Local") (`KismetMathLibrary.ClampVectorSize` (`SplineComponent.GetTangentAtDistanceAlongSpline` _spline_2 _returnvalue_6 "Local") 0.0 (`self.MeshLength`)) true)
        (`SceneComponent.K2_AttachToComponent` _returnvalue_4 (`self.Spline`) "None" "KeepRelative" "KeepRelative" "KeepRelative" true)
        (`SceneComponent.SetMobility` _returnvalue_4 (`self.Mobility`))))
    (else
      (for _index_2 (range (+ (- (`SplineComponent.GetNumberOfSplinePoints` _spline) 2) 1))
        (bind _returnvalue_7 (`KismetMaterialLibrary.CreateDynamicMaterialInstance` "/Game/Arada_Fajar/Materials/Master/Sequence_Mat1_Inst.Sequence_Mat1_Inst"))
        (bind _output_get (set `self.NewVar` _returnvalue_7))
        (bind _returnvalue_8 (`AddComponent|NODE_AddSplineMeshComponent-0`))
        (`SceneComponent.SetRelativeScale3D` _returnvalue_8 (`KismetMathLibrary.MakeVector` _cablesize _cablesize _cablesize))
        (`PrimitiveComponent.SetMaterial` _returnvalue_8 0 _output_get)
        (`MaterialInstanceDynamic.SetScalarParameterValue` _output_get "Speed" (`KismetMathLibrary.RandomFloatInRange` 0.4 0.6))
        (`StaticMeshComponent.SetStaticMesh` _returnvalue_8 (`self.New Mesh`))
        (`PrimitiveComponent.SetCollisionEnabled` _returnvalue_8 "QueryAndPhysics")
        (`SceneComponent.SetMobility` _returnvalue_8 (`self.New Mobility`))
        (`SceneComponent.K2_SetRelativeRotation` _returnvalue_8 (`self.Rotation`) false false)
        (`SceneComponent.K2_AttachToComponent` _returnvalue_8 (`self.DefaultSceneRoot`) "None" "KeepRelative" "KeepRelative" "KeepRelative" true)
        (`SplineMeshComponent.SetStartScale` _returnvalue_8 _returnvalue_2 true)
        (`SplineMeshComponent.SetEndScale` _returnvalue_8 _returnvalue_2 true)
        (bind (_location _tangent) (`SplineComponent.GetLocationAndTangentAtSplinePoint` _spline _index_2 "Local"))
        (bind (_location_2 _tangent_2) (`SplineComponent.GetLocationAndTangentAtSplinePoint` _spline (+ _index_2 1) "Local"))
        (`SplineMeshComponent.SetStartAndEnd` _returnvalue_8 _location _tangent _location_2 _tangent_2 true)
        (`SceneComponent.SetMobility` _returnvalue_8 (`self.Mobility`))))))