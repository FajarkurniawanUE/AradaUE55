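; BP_carBG is a background car that rides along a spline with a randomly picked skeletal mesh and matching animation.
; On BeginPlay, a Timeline scaled by Speed drives its position and rotation along the spline, and the car is re-randomized when the Timeline finishes.
; The construction script sets spotlight visibility from UseLight.
; The useLight? event is empty, leaving its runtime light and lamp-material logic disconnected.
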(event `useLight?`
  (params (Condition :type Boolean)))

(event `setRandomCar`
  (bind _animtoplay (break `SingleAnimationPlayData` (`|GetArrayItem` (`self.Animation Data`) (`self.RandomIndex`))))
  (bind _output_get (set `self.RandomIndex` (`KismetMathLibrary.RandomIntegerInRange` 0 (`KismetArrayLibrary.Array_LastIndex` (`self.CarSkeletalMesh`)))))
  (`self.useLight?` true)
  (`SkinnedMeshComponent.SetSkinnedAssetAndUpdate` (`self.SkeletalMesh`) (`|GetArrayItem` (`self.CarSkeletalMesh`) (`self.RandomIndex`)) false)
  (set `SkeletalMeshComponent.AnimationData` (make `SingleAnimationPlayData` _animtoplay true true 0.0 (`self.speed`)) (`self.SkeletalMesh`))
  (`SkeletalMeshComponent.SetAnimation` (`self.SkeletalMesh`) _animtoplay)
  (`SkeletalMeshComponent.Play` (`self.SkeletalMesh`) true)
  (`KismetSystemLibrary.PrintString` (`KismetStringLibrary.Conv_IntToString` _output_get)))

(event `self.ReceiveBeginPlay`
  (bind _spline (`self.Spline`))
  (`self.setRandomCar`)
  (`TimelineComponent.SetPlayRate` (`self.Timeline_0`) (`self.speed`))
  (bind (_direction _newtrack_0) (`Timeline|Timeline_0` :!via `PlayFromStart`)
    (:`Update`
      (bind _returnvalue (* (`SplineComponent.GetSplineLength` _spline) _newtrack_0))
      (`SceneComponent.K2_SetWorldTransform` (`self.SkeletalMesh`) (`KismetMathLibrary.MakeTransform` (`SplineComponent.GetLocationAtDistanceAlongSpline` _spline _returnvalue "World") (`SplineComponent.GetRotationAtDistanceAlongSpline` _spline _returnvalue "World")) false false))
    (:`Finished`
      (`self.setRandomCar`))))

(fn `UserConstructionScript`
  (`SceneComponent.SetVisibility` (`self.SpotLight1`) (`self.use light?`) false)
  (`SceneComponent.SetVisibility` (`self.SpotLight`) (`self.use light?`) false))