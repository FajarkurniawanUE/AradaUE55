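; Exit door interaction actor that lets the player interact with a specific door while looking at it in the interior scene.
; Tick compares the pc_arada controller's CurrentTracingActor to DoorSM, toggling this actor's input.
; Paired DoOnce gates reset each other, so the Umg_interior prompt and custom-depth highlight on two door meshes change only on trace transitions.
; Releasing Interact shows a list in that widget.
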(event `beingTrace`
  (`self.EnableInput` (`GameplayStatics.GetPlayerController` 0))
  (`|ExecutionSequence`
    (:`then_0`
      (`/Engine/EditorBlueprintResources/StandardMacros.DoOnce` false :!label _label
        (:`Completed`
          (bind _foundwidgets (`WidgetBlueprintLibrary.GetAllWidgetsOfClass` "/Game/Arada_Fajar/Blueprints/umg_interior.umg_interior_C" false))
          (`/Game/Arada_Fajar/Blueprints/umg_interior.show_interact` (`|GetArrayItem` _foundwidgets) "SelfHitTestInvisible")
          (`PrimitiveComponent.SetRenderCustomDepth` (`/Game/Arada_Fajar/Actors/Geometries/2b_door1.3BR_doors1_StaticMeshComponent0` (`self.Door SM`)) true)
          (`PrimitiveComponent.SetRenderCustomDepth` (`/Game/Arada_Fajar/Actors/Geometries/2b_door1.3BR_doors10_StaticMeshComponent0` (`self.Door SM`)) true))))
    (:`then_1`
      (goto _label_2 :!via `Reset`))))

(event `notTrace`
  (`self.DisableInput` (`GameplayStatics.GetPlayerController` 0))
  (`|ExecutionSequence`
    (:`then_0`
      (goto _label :!via `Reset`))
    (:`then_1`
      (`/Engine/EditorBlueprintResources/StandardMacros.DoOnce` false :!label _label_2
        (:`Completed`
          (bind _foundwidgets (`WidgetBlueprintLibrary.GetAllWidgetsOfClass` "/Game/Arada_Fajar/Blueprints/umg_interior.umg_interior_C" false))
          (`/Game/Arada_Fajar/Blueprints/umg_interior.show_interact` (`|GetArrayItem` _foundwidgets) "Collapsed")
          (`PrimitiveComponent.SetRenderCustomDepth` (`/Game/Arada_Fajar/Actors/Geometries/2b_door1.3BR_doors1_StaticMeshComponent0` (`self.Door SM`)) false)
          (`PrimitiveComponent.SetRenderCustomDepth` (`/Game/Arada_Fajar/Actors/Geometries/2b_door1.3BR_doors10_StaticMeshComponent0` (`self.Door SM`)) false))))))

(event `self.ReceiveTick`
  (params (DeltaSeconds :type "Float (single-precision)"))
  (bind _as2b_door_1 (cast `/Game/Arada_Fajar/Actors/Geometries/2b_door1` (`/Game/Arada_Fajar/Blueprints/pc_arada.CurrentTracingActor` (`self.As Pc Arada`)))
    (:`then`
      (if (== _as2b_door_1 (`self.Door SM`))
        (`self.beingTrace`)
        (else
          (`self.notTrace` :!label _label_3))))
    (:`CastFailed`
      (goto _label_3))))

(event `self.ReceiveBeginPlay`
  (`|ExecutionSequence`
    (:`then_2`
      (bind _aspc_arada (cast `/Game/Arada_Fajar/Blueprints/pc_arada` (`GameplayStatics.GetPlayerController` 0)))
      (set `self.As Pc Arada` _aspc_arada))))

(event `InputAction|Interact`
  (params (Key :type "Key Structure"))
  (:`Released`
    (bind _foundwidgets (`WidgetBlueprintLibrary.GetAllWidgetsOfClass` "/Game/Arada_Fajar/Blueprints/umg_interior.umg_interior_C" false))
    (`/Game/Arada_Fajar/Blueprints/umg_interior.show_list` (`|GetArrayItem` _foundwidgets) "Visible")))

(fn `UserConstructionScript`)