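; Building handler, attached to a StaticMeshActor, that fades the mesh to near-transparent and back on request.
; On BeginPlay it caches the original materials and builds translucent dynamic instances that copy their diffuse texture and color.
; settotranslucent swaps these in and a timeline lowers the Mask parameter; settodefault raises it back, then restores the originals.
; Paired DoOnce gates re-arm each other, so the two events only act alternately.
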(event `self.ReceiveBeginPlay`
  (`|ExecutionSequence`
    (:`then_0`
      (bind _asstatic_mesh_actor (cast `StaticMeshActor` (`self.GetAttachParentActor`)))
      (for _array_element (`MeshComponent.GetMaterials` (`StaticMeshActor.StaticMeshComponent` _asstatic_mesh_actor))
        (`KismetArrayLibrary.Array_Add` (`self.MaterialsDefault`) _array_element)))
    (:`then_1`
      (for _array_element_2 (`self.MaterialsDefault`)
        (bind _returnvalue (`KismetMaterialLibrary.CreateDynamicMaterialInstance` _array_element_2))
        (`KismetArrayLibrary.Array_Add` (`self.MaterialsDynamicProcess`) _returnvalue)))
    (:`then_2`
      (for _array_element_3 (`self.MaterialsDynamicProcess`)
        (bind _returnvalue_2 (`KismetMaterialLibrary.CreateDynamicMaterialInstance` "/Game/Arada_Fajar/Materials/Building/M_base_building_translucent.M_base_building_translucent"))
        (bind _returnvalue_3 (`MaterialInstanceDynamic.K2_GetTextureParameterValue` _array_element_3 "DiffuseTexture1"))
        (`MaterialInstanceDynamic.SetTextureParameterValue` _returnvalue_2 "DiffuseTexture1" _returnvalue_3)
        (bind _returnvalue_4 (`MaterialInstanceDynamic.K2_GetVectorParameterValue` _array_element_3 "Color1"))
        (`MaterialInstanceDynamic.SetVectorParameterValue` _returnvalue_2 "Color1" _returnvalue_4)
        (`KismetArrayLibrary.Array_Add` (`self.MaterialsDynamicTranslucent`) _returnvalue_2)))))

(event `set to translucent`
  (`/Engine/EditorBlueprintResources/StandardMacros.DoOnce` false :!label _label
    (:`Completed`
      (`|ExecutionSequence`
        (:`then_0`
          (bind _asstatic_mesh_actor (cast `StaticMeshActor` (`self.GetAttachParentActor`)))
          (for (_array_element _array_index) (`self.MaterialsDynamicTranslucent`)
            (bind _staticmeshcomponent (`StaticMeshActor.StaticMeshComponent` _asstatic_mesh_actor))
            (`PrimitiveComponent.SetMaterial` _staticmeshcomponent _array_index _array_element))
          (bind (_direction _newtrack_0) (`Timeline|Timeline` :!via `PlayFromStart`)
            (:`Update`
              (`MeshComponent.SetScalarParameterValueOnMaterials` _staticmeshcomponent "Mask" (`KismetMathLibrary.Lerp` 1.0 0.02 _newtrack_0)))))
        (:`then_1`
          (goto _label_2 :!via `Reset`))))))

(event `set to default`
  (`/Engine/EditorBlueprintResources/StandardMacros.DoOnce` false :!label _label_2
    (:`Completed`
      (`|ExecutionSequence`
        (:`then_0`
          (goto _label :!via `Reset`))
        (:`then_1`
          (bind _asstatic_mesh_actor (cast `StaticMeshActor` (`self.GetAttachParentActor`)))
          (bind (_direction _newtrack_0) (`Timeline|Timeline_0` :!via `PlayFromStart`)
            (:`Update`
              (`MeshComponent.SetScalarParameterValueOnMaterials` (`StaticMeshActor.StaticMeshComponent` _asstatic_mesh_actor) "Mask" (`KismetMathLibrary.Lerp` 0.02 1.0 _newtrack_0)))
            (:`Finished`
              (bind _asstatic_mesh_actor_2 (cast `StaticMeshActor` (`self.GetAttachParentActor`)))
              (for (_array_element _array_index) (`self.MaterialsDefault`)
                (`PrimitiveComponent.SetMaterial` (`StaticMeshActor.StaticMeshComponent` _asstatic_mesh_actor_2) _array_index _array_element)))))))))

(fn `UserConstructionScript`)