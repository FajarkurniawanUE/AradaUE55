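; Blueprint for a radial-blur post-process effect, currently inert because its Blurit event is empty and the blur logic is disconnected.
; The unconnected chain creates a dynamic instance of M_Base_RadianBlurPP_Inst and assigns it to the PostProcess settings as a full-weight blendable.
; A Timeline in that chain would then ramp the material's OverallBlur parameter through a Lerp to fade the blur.
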(event `Blurit`)

(fn `UserConstructionScript`)