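; Elevator interaction Blueprint that lets the player open the elevator menu from designated elevator meshes.
; Tick checks whether the player controller's traced StaticMeshActor is in ElevatorSM, toggling input accordingly.
; Paired DoOnce nodes re-arm each other, so the Umg_orbital interact prompt and custom-depth highlight update only when that state changes.
; Releasing Interact while input is enabled calls ShowElevatorMenu on the orbital widget.
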(event `beingTrace`
  (`self.EnableInput` (`GameplayStatics.GetPlayerController` 0))
  (`|ExecutionSequence`
    (:`then_0`
      (`/Engine/EditorBlueprintResources/StandardMacros.DoOnce` false :!label _label
        (:`Completed`
          (bind _foundwidgets (`WidgetBlueprintLibrary.GetAllWidgetsOfClass` "/Game/Arada_Fajar/Blueprints/umg_orbital.umg_orbital_C" false))
          (`/Game/Arada_Fajar/Blueprints/umg_orbital.showInteract` (`|GetArrayItem` _foundwidgets) "SelfHitTestInvisible")
          (`PrimitiveComponent.SetRenderCustomDepth` (`StaticMeshActor.StaticMeshComponent` (stale `self.ReceiveTick` _asstatic_mesh_actor)) true))))
    (:`then_1`
      (goto _label_2 :!via `Reset`))))

(event `notTrace`
  (`self.DisableInput` (`GameplayStatics.GetPlayerController` 0))
  (`|ExecutionSequence`
    (:`then_0`
      (goto _label :!via `Reset`))
    (:`then_1`
      (`/Engine/EditorBlueprintResources/StandardMacros.DoOnce` false :!label _label_2
        (:`Completed`
          (bind _foundwidgets (`WidgetBlueprintLibrary.GetAllWidgetsOfClass` "/Game/Arada_Fajar/Blueprints/umg_orbital.umg_orbital_C" false))
          (`/Game/Arada_Fajar/Blueprints/umg_orbital.showInteract` (`|GetArrayItem` _foundwidgets) "Collapsed")
          (for _array_element (`self.Elevator SM`)
            (`PrimitiveComponent.SetRenderCustomDepth` (`StaticMeshActor.StaticMeshComponent` _array_element) false)))))))

(event `self.ReceiveTick`
  (params (DeltaSeconds :type "Float (single-precision)"))
  (bind _asstatic_mesh_actor (cast `StaticMeshActor` (`/Game/Arada_Fajar/Blueprints/pc_arada.CurrentTracingActor` (`self.As Pc Arada`))))
  (if (`KismetArrayLibrary.Array_Contains` (`self.Elevator SM`) _asstatic_mesh_actor)
    (`self.beingTrace`)
    (else
      (`self.notTrace`))))

(event `self.ReceiveBeginPlay`
  (`|ExecutionSequence`
    (:`then_0`
      (bind _foundwidgets (`WidgetBlueprintLibrary.GetAllWidgetsOfClass` "/Game/Arada_Fajar/Blueprints/umg_orbital.umg_orbital_C" false))
      (set `self.umg_orbital` (`|GetArrayItem` _foundwidgets)))
    (:`then_1`
      (bind _aschar_arada_walk_exterior (cast `/Game/Arada_Fajar/Blueprints/char_arada_walk_exterior` (`GameplayStatics.GetPlayerCharacter` 0)))
      (set `self.As Char Arada Walk Exterior` _aschar_arada_walk_exterior))
    (:`then_2`
      (bind _aspc_arada (cast `/Game/Arada_Fajar/Blueprints/pc_arada` (`GameplayStatics.GetPlayerController` 0)))
      (set `self.As Pc Arada` _aspc_arada))))

(event `InputAction|Interact`
  (params (Key :type "Key Structure"))
  (:`Released`
    (bind _foundwidgets (`WidgetBlueprintLibrary.GetAllWidgetsOfClass` "/Game/Arada_Fajar/Blueprints/umg_orbital.umg_orbital_C" false))
    (`/Game/Arada_Fajar/Blueprints/umg_orbital.showElevatorMenu` (`|GetArrayItem` _foundwidgets))))

(fn `UserConstructionScript`)