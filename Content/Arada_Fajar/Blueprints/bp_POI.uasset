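; Point-of-interest actor that shows or hides its Widget component according to UI state and line of sight to the orbital pawn's camera.
; BeginPlay caches the player's pawn_arada_orbital.
; Each Tick hides the widget when HideUI or WalkMode is set or a Visibility trace from widget to camera is blocked, otherwise shows it.
; Two DoOnce gates reset each other so visibility is set only when the state changes.
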(event `self.ReceiveTick`
  (params (DeltaSeconds :type "Float (single-precision)"))
  (bind _widget (`self.Widget`))
  (if (`self.HideUI`)
    (`|ExecutionSequence` :!label _label
      (:`then_0`
        (`/Engine/EditorBlueprintResources/StandardMacros.DoOnce` false :!label _label_2
          (:`Completed`
            (`SceneComponent.SetVisibility` _widget false false))))
      (:`then_1`
        (goto _label_3 :!via `Reset`)))
    (elif (`self.WalkMode`)
      (goto _label)
      (else
        (bind (_outhit _returnvalue) (`KismetSystemLibrary.LineTraceSingle` (`SceneComponent.K2_GetComponentLocation` (`self.Widget`)) (`SceneComponent.K2_GetComponentLocation` (`/Game/Arada_Fajar/Blueprints/pawn_arada_orbital.Camera` (`self.As Pawn Arada Orbital`))) "TraceTypeQuery1"))
        (if _returnvalue
          (goto _label)
          (else
            (`|ExecutionSequence`
              (:`then_0`
                (goto _label_2 :!via `Reset`))
              (:`then_1`
                (`/Engine/EditorBlueprintResources/StandardMacros.DoOnce` false :!label _label_3
                  (:`Completed`
                    (`SceneComponent.SetVisibility` _widget true false)))))))))))

(event `self.ReceiveBeginPlay`
  (bind _aspawn_arada_orbital (cast `/Game/Arada_Fajar/Blueprints/pawn_arada_orbital` (`GameplayStatics.GetPlayerPawn` 0)))
  (set `self.As Pawn Arada Orbital` _aspawn_arada_orbital))

(fn `UserConstructionScript`)