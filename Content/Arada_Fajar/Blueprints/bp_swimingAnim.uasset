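; Actor that animates a Swimming component travelling along a spline in a continuous loop.
; Each tick advances a distance by Speed and delta time, then sets the component's relative transform from the spline's local transform at that point.
; A yaw offset corrects the facing and a fixed uniform scale is applied.
; The distance resets to zero once it exceeds the spline length.
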(event `self.ReceiveTick`
  (params (DeltaSeconds :type "Float (single-precision)"))
  (bind (_returnvalue_location _returnvalue_rotation) (`KismetMathLibrary.BreakTransform` (`SplineComponent.GetTransformAtDistanceAlongSpline` (`self.Spline`) (`self.NewDistance`) "Local" false)))
  (set `self.NewDistance` (+ (* DeltaSeconds (`self.Speed`)) (`self.NewDistance`)))
  (`SceneComponent.K2_SetRelativeTransform` (`self.Swimming`) (`KismetMathLibrary.MakeTransform` _returnvalue_location (`KismetMathLibrary.MakeRotator` (.roll _returnvalue_rotation) (.pitch _returnvalue_rotation) (+ (.yaw _returnvalue_rotation) -90.0)) (5.0 5.0 5.0)) false false)
  (if (> (`self.NewDistance`) (`SplineComponent.GetSplineLength` (`self.Spline`)))
    (set `self.NewDistance` 0.0)))

(fn `UserConstructionScript`)