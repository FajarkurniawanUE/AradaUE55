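; BP_carBG_spline spawns a list of actors, apparently background cars, and drives them in a loop along a spline.
; On BeginPlay, SpawnActors spaces the ActorList classes evenly by spline length and stores a randomly jittered distance for each in SpawnedActorMap.
; Each Tick, MoveActors advances every stored distance by Speed times delta time, snaps the actor to that spline transform and restarts at zero past the end.
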(event `self.ReceiveBeginPlay`
  (`self.SpawnActors`))

(event `self.ReceiveTick`
  (params (DeltaSeconds :type "Float (single-precision)"))
  (bind _spawnedactormap (`self.SpawnedActorMap`))
  (bind _keys (`BlueprintMapLibrary.Map_Keys` _spawnedactormap))
  (for _array_element _keys
    (`self.MoveActors` _array_element (`BlueprintMapLibrary.Map_Find` _spawnedactormap _array_element))))

(fn `MoveActors`
  (params (inActor :type "Actor Object Reference") (inDistance :type "Float (double-precision)"))
  (locals (NewDistance :type "Float (double-precision)"))
  (bind _spline (`self.Spline`))
  (bind _output_get (set `local.NewDistance` (+ inDistance (* (`self.Speed`) (`GameplayStatics.GetWorldDeltaSeconds`)))))
  (if (>= _output_get (`SplineComponent.GetSplineLength` _spline))
    (set `local.NewDistance` 0.0))
  (`self.K2_SetActorTransform` inActor (`SplineComponent.GetTransformAtDistanceAlongSpline` _spline (`local.NewDistance`) "World" false) false false)
  (`BlueprintMapLibrary.Map_Add` (`self.SpawnedActorMap`) inActor (`local.NewDistance`)))

(fn `SpawnActors`
  (locals (SplitDistance :type "Float (double-precision)") (InitDistance :type "Float (double-precision)"))
  (bind _returnvalue (`KismetArrayLibrary.Array_Length` (`self.ActorList`)))
  (bind _returnvalue_2 (/ (`local.SplitDistance`) 2.0))
  (if (> _returnvalue 0)
    (bind _output_get (set `local.SplitDistance` (/ (`SplineComponent.GetSplineLength` (`self.Spline`)) _returnvalue)))
    (for (_array_element _array_index) (`self.ActorList`)
      (set `local.InitDistance` (* _array_index _output_get))
      (bind _returnvalue_3 (`|SpawnActorFromClass` _array_element (`SplineComponent.GetTransformAtDistanceAlongSpline` (`self.Spline`) (`local.InitDistance`) "World" false) "Undefined" "MultiplyWithRoot" null null))
      (`BlueprintMapLibrary.Map_Add` (`self.SpawnedActorMap`) _returnvalue_3 (`KismetMathLibrary.RandomFloatInRange` (+ (`local.InitDistance`) _returnvalue_2) (- (`local.InitDistance`) _returnvalue_2))))))

(fn `UserConstructionScript`)